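; First-person player character Blueprint that handles looking, movement, jumping and smooth crouching.
; Look axes feed clamped controller pitch and yaw, while movement follows only the yaw of the control rotation.
; Holding Crouch plays a timeline that lerps the capsule half height from its BeginPlay value to the movement component's crouched height, and releasing reverses it.
; Crouching sets an IsCrouching flag rather than calling the built-in Crouch.
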(event Custom|StartCrouch
  (Variables|Default|SetIsCrouching true)
  (bind _lerpvalue (Timeline|CrouchSmooth Play)
    (:Update
      (Components|Capsule|SetCapsuleHalfHeight (Variables|Collision|GetCapsuleComponent) (Math|Float|Lerp (Variables|Default|GetCapsuleHalfHeight) (Variables|/Script/Engine.CharacterMovementComponent|GetCrouchedHalfHeight (Variables|Character|GetCharacterMovement)) _lerpvalue) true))))

(event Custom|StopCrouch
  (Variables|Default|SetIsCrouching false)
  (bind _lerpvalue (Timeline|CrouchSmooth Reverse)
    (:Update
      (Components|Capsule|SetCapsuleHalfHeight (Variables|Collision|GetCapsuleComponent) (Math|Float|Lerp (Variables|Default|GetCapsuleHalfHeight) (Variables|/Script/Engine.CharacterMovementComponent|GetCrouchedHalfHeight (Variables|Character|GetCharacterMovement)) _lerpvalue) true))))

(event EventBeginPlay
  (Variables|Default|SetCapsuleHalfHeight (Variables|/Script/Engine.CapsuleComponent|GetCapsuleHalfHeight (Variables|Collision|GetCapsuleComponent))))

(event Input|ActionEvents|InputActionJump
  (params (Key :type Key%20Structure :default "None"))
  (:Pressed
    (Character|Jump)))

(event Input|ActionEvents|InputActionCrouch
  (params (Key :type Key%20Structure :default "None"))
  (:Pressed
    (CallFunction|StartCrouch))
  (:Released
    (CallFunction|StopCrouch)))

(event Input|AxisEvents|InputAxisForward/Backward
  (params (AxisValue :type Float%20%28single-precision%29))
  ;[1 1 1] Basic Movment
  (Pawn|Input|AddMovementInput (Math|Vector|GetForwardVector (Math|Rotator|MakeRotator 0.0 0.0 (.Yaw (Math|Rotator|BreakRotator (Pawn|GetControlRotation :!class /Script/Engine.Pawn))))) AxisValue false))

(event Input|AxisEvents|InputAxisRight/Left
  (params (AxisValue :type Float%20%28single-precision%29))
  ;[1 1 1] Basic Movment
  (Pawn|Input|AddMovementInput (Math|Vector|GetRightVector (Math|Rotator|MakeRotator 0.0 0.0 (.Yaw (Math|Rotator|BreakRotator (Pawn|GetControlRotation :!class /Script/Engine.Pawn))))) AxisValue false))

(event Input|AxisEvents|InputAxisLookUp/LookDown
  (params (AxisValue :type Float%20%28single-precision%29))
  ;[1 1 1] Camera Rotation (Looking)
  (Pawn|Input|AddControllerPitchInput (Math|Float|Clamp(Float) AxisValue -1.0)))

(event Input|AxisEvents|InputAxisLookRight/LookLeft
  (params (AxisValue :type Float%20%28single-precision%29))
  ;[1 1 1] Camera Rotation (Looking)
  (Pawn|Input|AddControllerYawInput (Math|Float|Clamp(Float) AxisValue -1.0)))

(fn ConstructionScript)